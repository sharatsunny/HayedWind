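; BP_RotatableRoom is a grid maze room generator, though its construction script is empty and the generation chains are disconnected.
; Border indices seed a flattened square grid, where a seeded random walk carves path and bridge tiles two cells at a time.
; Dead ends backtrack while bridges convert to paths, then remaining cells become walls.
; A spawn macro maps indices to hierarchical instanced meshes for border and path tiles; no rotation logic exists.
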(event EventBeginPlay)

(event Collision|EventActorBeginOverlap
  (params (OtherActor :type Actor%20Object%20Reference)))

(event EventTick
  (params (DeltaSeconds :type Float%20%28single-precision%29)))

(fn ConstructionScript)

(fn PopulateBorder
  (params (Size :type Integer) (BorderArray :type Array%20of%20Integers))
  (LocalVariables|SetLSize Size)
  ;[1 1 1] NorthBorder
  (for _index (range 0 (- (LocalVariables|GetLSize) 1))
    (Utilities|Array|Add BorderArray _index))
  ;[1 1 1] EastBorder
  (for _index_2 (range 0 (- (LocalVariables|GetLSize) 2))
    (Utilities|Array|Add BorderArray (+ (* _index_2 (LocalVariables|GetLSize)) (- (LocalVariables|GetLSize) 1))))
  ;[1 1 1] SouthBorder
  (for _index_3 (range 0 (LocalVariables|GetLSize))
    (Utilities|Array|Add BorderArray (+ (- _index_3 1) (* (LocalVariables|GetLSize) (- (LocalVariables|GetLSize) 1)))))
  ;[1 1 1] WestBorder
  (for _index_4 (range 0 (- (LocalVariables|GetLSize) 2))
    (Utilities|Array|Add BorderArray (* _index_4 (LocalVariables|GetLSize)))))

(fn SetInitialTile
  (Variables|Default|SetCurrentTile (+ (Variables|Default|GetSize) 1))
  (Utilities|Array|Add (Variables|Default|GetPathTiles) (Variables|Default|GetCurrentTile)))

(fn AddBridgeandPathTile
  (params (PathTile :type Integer%20%28by%20ref%29) (BridgeTile :type Integer%20%28by%20ref%29))
  (Utilities|Array|Add (Variables|Default|GetPathTiles) PathTile)
  (Variables|Default|SetCurrentTile PathTile)
  (Utilities|Array|Add (Variables|Default|GetBridgeTiles) BridgeTile))

(fn PickNearbyTile
  (bind _size (Variables|Default|GetSize))
  (bind _currenttile (Variables|Default|GetCurrentTile))
  (bind _currenttile_2 (Variables|Default|GetCurrentTile))
  (bind _size_2 (Variables|Default|GetSize))
  (bind _currenttile_3 (Variables|Default|GetCurrentTile))
  (bind _currenttile_4 (Variables|Default|GetCurrentTile))
  (bind (_btileinarray_ _pathtile _bridgetile) (Utilities|CheckNorthTile _currenttile _size true))
  (bind (_btileinarray__2 _pathtile_2 _bridgetile_2) (Utilities|CheckEastTile _currenttile_2 true))
  (bind (_btileinarray__3 _pathtile_3 _bridgetile_3) (Utilities|CheckNorthTile _currenttile_3 _size_2 false))
  (bind (_btileinarray__4 _pathtile_4 _bridgetile_4) (Utilities|CheckEastTile _currenttile_4 false))
  (switch int (Math|Random|RandomIntegerinRangefromStream 0 3 (Variables|Default|GetRandomStream))
    (:0
      (if _btileinarray__3 :!label _label
        (Utilities|CycleCounter (Variables|Default|GetCycle%20Counter) 4
          (:True
            (if _btileinarray_ :!label _label_2
              (Utilities|CycleCounter (Variables|Default|GetCycle%20Counter) 4
                (:True
                  (if _btileinarray__4 :!label _label_3
                    (Utilities|CycleCounter (Variables|Default|GetCycle%20Counter) 4
                      (:True
                        (if _btileinarray__2 :!label _label_4
                          (Utilities|CycleCounter (Variables|Default|GetCycle%20Counter) 4
                            (:True
                              (goto _label))
                            (:False
                              (Variables|Default|SetbCurrentSideFree? false :!label _label_5)))
                          (else
                            (CallFunction|AddBridgeandPathTile _pathtile_2 _bridgetile_2))))
                      (:False
                        (goto _label_5)))
                    (else
                      (CallFunction|AddBridgeandPathTile _pathtile_4 _bridgetile_4))))
                (:False
                  (goto _label_5)))
              (else
                (CallFunction|AddBridgeandPathTile _pathtile _bridgetile))))
          (:False
            (goto _label_5)))
        (else
          (CallFunction|AddBridgeandPathTile _pathtile_3 _bridgetile_3))))
    (:1
      (goto _label_3))
    (:2
      (goto _label_2))
    (:3
      (goto _label_4)))
  (return))

(fn BackTrack
  (bind _array_element (Utilities|RevforEachLoopwithBreak (Variables|Default|GetPathTiles) :!label _label)
    (:LoopBody
      (if (not (Utilities|Array|ContainsItem (Variables|Default|GetCheckedTiles) _array_element))
        (Variables|Default|SetCurrentTile _array_element)
        (goto _label Break)))))

(fn PopulateWalls
  (bind _size (Variables|Default|GetSize))
  (for _index (range 0 (- (* _size _size) 1))
    (if (not (Utilities|CheckTilesArray _index))
      (Utilities|Array|Add (Variables|Default|GetWallTiles) _index))))