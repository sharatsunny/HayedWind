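; BP_RotatableRoom is a room actor that tilts in roll and pitch from X and Y input values.
; SetRotation, while KeyPressed is true, scales the inputs by RotSpeed, inverts pitch and combines the result with the current actor rotation.
; It clamps all three axes between RotMin and RotMax, applies them as relative rotation and prints the unclamped rotation for debugging.
; The event graph and construction script are empty.
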(event EventBeginPlay)

(event Collision|EventActorBeginOverlap
  (params (OtherActor :type Actor%20Object%20Reference)))

(event EventTick
  (params (DeltaSeconds :type Float%20%28single-precision%29)))

(fn ConstructionScript)

(fn SetRotation
  (params (XRotation :type Float%20%28single-precision%29) (YRotation :type Float%20%28single-precision%29) (KeyPressed? :type Boolean))
  (bind _returnvalue (Transformation|GetActorRotation))
  (bind _rotmin (Variables|Default|GetRotMin))
  (bind _rotspeed (Variables|Default|GetRotSpeed))
  (bind _rotmax (Variables|Default|GetRotMax))
  (bind _returnvalue_2 (* YRotation _rotspeed))
  (bind _returnvalue_3 (* XRotation _rotspeed))
  (bind _returnvalue_4 (* _returnvalue_2 -1.0))
  (bind _returnvalue_5 (Math|Rotator|MakeRotator _returnvalue_3 _returnvalue_4 0.0))
  (bind _returnvalue_6 (Math|Rotator|CombineRotators _returnvalue _returnvalue_5))
  (bind (_roll _pitch _yaw) (Math|Rotator|BreakRotator _returnvalue_6))
  (if KeyPressed?
    (Transformation|SetActorRelativeRotation (Math|Rotator|MakeRotator (Math|Float|ClampAngle _roll _rotmin _rotmax) (Math|Float|ClampAngle _pitch _rotmin _rotmax) (Math|Float|ClampAngle _yaw _rotmin _rotmax)))
    (Development|PrintString (Utilities|String|ToString(Rotator) _returnvalue_6))
    (return)))