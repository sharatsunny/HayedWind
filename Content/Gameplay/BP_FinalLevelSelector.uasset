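; BP_FinalLevelSelector is a trigger volume that sends the player to the good or bad ending level.
; On overlap by ThirdPersonCharacter, it compares the game instance's elapsed time with a limit to pick the ending.
; Unless already in that level, it fades out camera and audio, then opens it after a delay.
; It also saves the next level index as unlocked, using a newly created GameJam_Save rather than a loaded one.
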(event OnComponentBeginOverlap(Box)
  (params (OverlappedComponent :type Primitive%20Component%20Object%20Reference) (OtherActor :type Actor%20Object%20Reference) (OtherComp :type Primitive%20Component%20Object%20Reference) (OtherBodyIndex :type Integer) (bFromSweep :type Boolean) (SweepResult :type Hit%20Result%20Structure%20%28by%20ref%29))
  (bind _badendlevel (Variables|Default|GetBadEndLevel))
  (bind _goodendlevel (Variables|Default|GetGoodEndLevel))
  (bind _timelimittillbadend (Variables|Default|GetTimeLimitTillBadEnd))
  (bind _fadeduration (Variables|Default|GetFadeDuration))
  (bind _nextlevelindex (Variables|Default|GetNextLevelIndex))
  (bind _gameinstref (Variables|Default|GetGameInstRef))
  (bind _gametimeinseconds (Variables|/Game/GameJam_Instance.GameJam_Instance_C|GetGameTimeInSeconds _gameinstref))
  (bind _returnvalue (Math|Float|Truncate _gametimeinseconds))
  (bind _returnvalue_2 (> _returnvalue _timelimittillbadend))
  (bind _returnvalue_3 (select _returnvalue_2 _badendlevel _goodendlevel))
  (Utilities|Casting|CastToThirdPersonCharacter OtherActor)
  (bind _returnvalue_4 (Game|GetCurrentLevelName true))
  (if (Utilities|Enum|Equal(Enum) _returnvalue_4 (Utilities|String|ToString(Name) _returnvalue_3))
    _
    (else
      (CameraFades|StartCameraFade :self (Game|GetPlayerCameraManager 0) :ToAlpha 1.0 :Duration _fadeduration :bShouldFadeAudio true :bHoldWhenFinished true)
      (Utilities|FlowControl|Delay _fadeduration)
      (Game|OpenLevel(byName) _returnvalue_3)))
  (bind _returnvalue_5 (SaveGame|CreateSaveGameObject "/Game/GameJam_Save.GameJam_Save_C"))
  (bind _asgame_jam_save (Utilities|Casting|CastToGameJam_Save _returnvalue_5))
  (if (Utilities|Set|Contains (Variables|/Game/GameJam_Save.GameJam_Save_C|GetLevelUnlocked _asgame_jam_save) _nextlevelindex)
    _
    (else
      (Utilities|Set|Add (Variables|/Game/GameJam_Save.GameJam_Save_C|GetLevelUnlocked _asgame_jam_save) _nextlevelindex)))
  (SaveGame|SaveGametoSlot _asgame_jam_save (Utilities|String|ToString(Name) (Variables|/Game/GameJam_Save.GameJam_Save_C|GetSlotName _asgame_jam_save))))

(event EventBeginPlay
  (bind _asgame_jam_instance (Utilities|Casting|CastToGameJam_Instance (Game|GetGameInstance)))
  (Variables|Default|SetGameInstRef _asgame_jam_instance))

(event Collision|EventActorBeginOverlap
  (params (OtherActor :type Actor%20Object%20Reference)))

(event EventTick
  (params (DeltaSeconds :type Float%20%28single-precision%29)))

(fn ConstructionScript)