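; A launcher volume that flings the third-person character into the air when jump is pressed inside its box.
; Entering the box stores the player and starts a very fast looping timer that polls the jump input, and leaving clears it.
; The launch overrides velocity, pushing along the follow camera's forward vector, scaled by half the player's distance to NewLoc, plus LaunchHeight upward.
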(event OnComponentBeginOverlap(Box)
  (params (OverlappedComponent :type Primitive%20Component%20Object%20Reference) (OtherActor :type Actor%20Object%20Reference) (OtherComp :type Primitive%20Component%20Object%20Reference) (OtherBodyIndex :type Integer) (bFromSweep :type Boolean) (SweepResult :type Hit%20Result%20Structure%20%28by%20ref%29))
  (bind _asthird_person_character (Utilities|Casting|CastToThirdPersonCharacter OtherActor))
  (Variables|Default|SetPlayerRef _asthird_person_character)
  (bind _returnvalue (Utilities|Time|SetTimerbyFunctionName 0 "CheckLaunch" 0.001 true)))

(event OnComponentEndOverlap(Box)
  (params (OverlappedComponent :type Primitive%20Component%20Object%20Reference) (OtherActor :type Actor%20Object%20Reference) (OtherComp :type Primitive%20Component%20Object%20Reference) (OtherBodyIndex :type Integer))
  (Utilities|Casting|CastToThirdPersonCharacter OtherActor)
  (Utilities|Time|ClearandInvalidateTimerbyHandle (stale OnComponentBeginOverlap(Box) _returnvalue)))

(event Custom|CheckLaunch
  (bind _playerref (Variables|Default|GetPlayerRef))
  (if (Variables|/Game/ThirdPersonBP/Blueprints/ThirdPersonCharacter.ThirdPersonCharacter_C|GetJumpPressed _playerref)
    (Character|LaunchCharacter _playerref (+ (* (Math|Vector|GetForwardVector (Transformation|GetWorldRotation (Variables|/Game/ThirdPersonBP/Blueprints/ThirdPersonCharacter.ThirdPersonCharacter_C|GetFollowCamera _playerref))) (/ (Math|Vector|VectorLength (- (Transformation|GetActorLocation _playerref) (Variables|Default|GetNewLoc))) 2.0)) (Math|Vector|MakeVector 0.0 0.0 (Variables|Default|GetLaunchHeight))) true true)))

(event EventBeginPlay)

(event Collision|EventActorBeginOverlap
  (params (OtherActor :type Actor%20Object%20Reference)))

(event EventTick
  (params (DeltaSeconds :type Float%20%28single-precision%29)))

(fn ConstructionScript)