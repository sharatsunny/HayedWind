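; Configurable moving hazard that travels along control points and damages any ThirdPersonCharacter entering its box.
; The construction script applies the chosen mesh and transform, then sizes the box from the mesh bounds.
; On BeginPlay, exposed path, duration and behaviour settings are copied into an InterpToMovement component and finalised.
; SetSpeed changes pace by adding scaled input to the actor's CustomTimeDilation, clamped between given limits.
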(event OnComponentBeginOverlap(Box)
  (params (OverlappedComponent :type Primitive%20Component%20Object%20Reference) (OtherActor :type Actor%20Object%20Reference) (OtherComp :type Primitive%20Component%20Object%20Reference) (OtherBodyIndex :type Integer) (bFromSweep :type Boolean) (SweepResult :type Hit%20Result%20Structure%20%28by%20ref%29))
  (bind _asthird_person_character (Utilities|Casting|CastToThirdPersonCharacter OtherActor))
  (Game|Damage|ApplyDamage _asthird_person_character (Variables|Default|GetDamageToPlayer) 0 0))

(event EventBeginPlay
  (bind _interptomovement (Variables|Default|GetInterpToMovement))
  (Variables|/Script/Engine.InterpToMovementComponent|SetDuration _interptomovement (Variables|Movement|GetDuration))
  (Variables|/Script/Engine.InterpToMovementComponent|SetControlPoints _interptomovement (Variables|Movement|GetControlPoints))
  (Variables|/Script/Engine.InterpToMovementComponent|SetbPauseOnImpact _interptomovement (Variables|Movement|GetPauseOnImpact))
  (Variables|/Script/Engine.InterpToMovementComponent|SetBehaviourType _interptomovement (Variables|Movement|GetBehaviourType))
  (Class|InterptoMovementComponent|FinaliseControlPoints _interptomovement))

(event Collision|EventActorBeginOverlap
  (params (OtherActor :type Actor%20Object%20Reference)))

(event EventTick
  (params (DeltaSeconds :type Float%20%28single-precision%29)))

(fn ConstructionScript
  (bind _staticmesh (Variables|Default|GetStaticMesh))
  (Components|StaticMesh|SetStaticMesh _staticmesh (Variables|StaticMesh|GetNewStaticMesh))
  (Transformation|SetRelativeTransform _staticmesh (Variables|StaticMesh|GetRelativeTransform) false false)
  (Components|Box|SetBoxExtent (Variables|Default|GetBox) (.BoxExtent (Collision|GetComponentBounds _staticmesh)) true))

(fn SetSpeed
  (params (YInput :type Float%20%28single-precision%29) (MaxSpeed :type Float%20%28single-precision%29) (MinSpeed :type Float%20%28single-precision%29))
  (Variables|Default|SetCustomTimeDilation (select (< (+ (Variables|Default|GetCustomTimeDilation) (* YInput (Variables|Default|GetSpeed))) MinSpeed) MinSpeed (select (> (+ (Variables|Default|GetCustomTimeDilation) (* YInput (Variables|Default|GetSpeed))) MaxSpeed) MaxSpeed (+ (Variables|Default|GetCustomTimeDilation) (* YInput (Variables|Default|GetSpeed)))))))