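; Falling platform that shakes when a ThirdPersonCharacter touches it, drops after a time limit, then respawns.
; Box overlap starts a looping ShakeObject timer that randomly jitters location and rotation, then interpolates the actor 1000 units down its up axis.
; A dynamic material's Alpha fades out after the fall; DelayClearing and ResetPlatform timers then restore the original transform and fade it back in.
; Construction script sets the mesh and sizes the trigger box from its bounds.
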(event OnComponentBeginOverlap(Box)
  (params (OverlappedComponent :type Primitive%20Component%20Object%20Reference) (OtherActor :type Actor%20Object%20Reference) (OtherComp :type Primitive%20Component%20Object%20Reference) (OtherBodyIndex :type Integer) (bFromSweep :type Boolean) (SweepResult :type Hit%20Result%20Structure%20%28by%20ref%29))
  (Utilities|Casting|CastToThirdPersonCharacter OtherActor
    (:then
      (bind _returnvalue (Utilities|Time|SetTimerbyFunctionName 0 "ShakeObject" 0.001 true)))
    (:CastFailed
      (Development|PrintString "Hello"))))

(event OnComponentEndOverlap(Box)
  (params (OverlappedComponent :type Primitive%20Component%20Object%20Reference) (OtherActor :type Actor%20Object%20Reference) (OtherComp :type Primitive%20Component%20Object%20Reference) (OtherBodyIndex :type Integer))
  (Utilities|Casting|CastToThirdPersonCharacter OtherActor
    (:then
      (if (> (Variables|Default|GetLocalTimer) (Variables|Delays|GetTimeAllowedOnPlatform))
        (if (Variables|Default|GetPlatformFell)
          (Utilities|Time|ClearandInvalidateTimerbyHandle (stale OnComponentBeginOverlap(Box) _returnvalue))
          (Utilities|Time|ClearandInvalidateTimerbyHandle (stale Custom|ShakeObject _returnvalue_4))
          (Utilities|FlowControl|Delay (Variables|Delays|GetDelayBeforeResettingPlatform))
          (bind _returnvalue (Utilities|Time|SetTimerbyFunctionName 0 "ResetPlatform" 0.001 true))
          (else
            (Utilities|FlowControl|Delay 0.2)))))
    (:CastFailed
      (Development|PrintString "Hello"))))

(event Custom|ResetPlatform
  (bind _dynamicmatref (Variables|Default|GetDynamicMatRef))
  (Variables|Default|SetLocalTimer 0.0)
  (Transformation|SetActorLocationAndRotation (Variables|Location|GetOGloc) (Variables|Location|GetOGRot))
  (bind _returnvalue (Rendering|Material|GetScalarParameterValue _dynamicmatref "Alpha" :!class /Script/Engine.MaterialInstanceDynamic))
  (Rendering|Material|SetScalarParameterValue _dynamicmatref "Alpha" (Math|Interpolation|FInterptoConstant _returnvalue 1.0 (Utilities|Time|GetWorldDeltaSeconds) (Variables|Default|GetAlphaSpeed)) :!class /Script/Engine.MaterialInstanceDynamic)
  (if (== _returnvalue 1.0)
    (Utilities|Time|ClearandInvalidateTimerbyHandle (stale OnComponentEndOverlap(Box) _returnvalue))))

(event Custom|ShakeObject
  (bind _randomrotmin (Variables|Rotation|GetRandomRotMin))
  (bind _randomrotmax (Variables|Rotation|GetRandomRotMax))
  (bind _dynamicmatref (Variables|Default|GetDynamicMatRef))
  (bind _rotation (Variables|Rotation|GetRotation))
  (bind _location (Variables|Location|GetLocation))
  (bind _randomlocmin (Variables|Location|GetRandomLocMin))
  (bind _randomlocmax (Variables|Location|GetRandomLocMax))
  (bind (_x _y _z) (Math|Vector|BreakVector _location))
  (bind _returnvalue (Math|Random|RandomFloatinRange _randomlocmin _randomlocmax))
  (bind (_roll _pitch _yaw) (Math|Rotator|BreakRotator _rotation))
  (bind _returnvalue_2 (Math|Random|RandomFloatinRange _randomrotmin _randomrotmax))
  (Variables|Default|SetLocalTimer (+ (Utilities|Time|GetWorldDeltaSeconds) (Variables|Default|GetLocalTimer)))
  (if (> (Variables|Default|GetLocalTimer) (Variables|Delays|GetTimeAllowedOnPlatform))
    (Transformation|SetActorLocation (Math|Interpolation|VInterptoConstant (Transformation|GetActorLocation) (Variables|Default|GetFallLocation) (Utilities|Time|GetWorldDeltaSeconds) (Variables|Delays|GetInterpSpeed)) false false)
    (if (Math|Vector|Equal(Vector) (Transformation|GetActorLocation) (Variables|Default|GetFallLocation) 0.1)
      (bind _returnvalue_3 (Rendering|Material|GetScalarParameterValue _dynamicmatref "Alpha" :!class /Script/Engine.MaterialInstanceDynamic))
      (Rendering|Material|SetScalarParameterValue _dynamicmatref "Alpha" (Math|Interpolation|FInterptoConstant _returnvalue_3 0.0 (Utilities|Time|GetWorldDeltaSeconds) (Variables|Default|GetAlphaSpeed)) :!class /Script/Engine.MaterialInstanceDynamic)
      (if (== _returnvalue_3 0.0)
        (Variables|Default|SetPlatformFell true)
        (bind _returnvalue_4 (Utilities|Time|SetTimerbyFunctionName 0 "DelayClearing" 0.001 true))
        (else
          (Variables|Default|SetPlatformFell false :!label _label)))
      (else
        (goto _label)))
    (else
      (Transformation|SetActorLocationAndRotation (Math|Interpolation|VInterptoConstant (Transformation|GetActorLocation) (Math|Vector|MakeVector (+ _x _returnvalue) (+ _y _returnvalue) _z) (Utilities|Time|GetWorldDeltaSeconds) (Variables|Delays|GetInterpSpeed)) (Class|KismetMathLibrary|RInterptoConstant (Transformation|GetActorRotation) (Math|Rotator|MakeRotator (+ _roll _returnvalue_2) (+ _pitch _returnvalue_2) (+ _yaw _returnvalue_2)) (Utilities|Time|GetWorldDeltaSeconds) (Variables|Delays|GetInterpSpeed))))))

(event Custom|DelayClearing
  (if (> (Variables|Default|GetLocalTimer) (Variables|Delays|GetTimeAllowedOnPlatform))
    (if (Variables|Default|GetPlatformFell)
      (Utilities|Time|ClearandInvalidateTimerbyHandle (stale OnComponentBeginOverlap(Box) _returnvalue))
      (Utilities|Time|ClearandInvalidateTimerbyHandle (stale Custom|ShakeObject _returnvalue_4))
      (Utilities|FlowControl|Delay (Variables|Delays|GetDelayBeforeResettingPlatform))
      (bind _returnvalue (Utilities|Time|SetTimerbyFunctionName 0 "ResetPlatform" 0.001 true))
      (else
        (Utilities|FlowControl|Delay 0.2)))))

(event EventBeginPlay
  (bind _returnvalue (Transformation|GetActorLocation))
  (bind _returnvalue_2 (Transformation|GetActorRotation))
  (bind _meshmaterial (Variables|Default|GetMeshMaterial))
  (bind _staticmesh (Variables|Default|GetStaticMesh))
  (Variables|Rotation|SetRotation _returnvalue_2)
  (Variables|Location|SetOGRot _returnvalue_2)
  (Variables|Location|SetLocation _returnvalue)
  (Variables|Location|SetOGloc _returnvalue)
  (Variables|Default|SetFallLocation (+ _returnvalue (* (Transformation|GetActorUpVector) -1e+03)))
  (Rendering|Material|SetMaterial _staticmesh 0 _meshmaterial)
  (bind _returnvalue_3 (Rendering|Material|CreateDynamicMaterialInstance _staticmesh 0 _meshmaterial "None" :!class /Script/Engine.PrimitiveComponent))
  (bind _output_get (Variables|Default|SetDynamicMatRef _returnvalue_3))
  (Rendering|Material|GetScalarParameterValue _output_get "Alpha" :!class /Script/Engine.MaterialInstanceDynamic))

(fn ConstructionScript
  (bind _staticmesh (Variables|Default|GetStaticMesh))
  (Components|StaticMesh|SetStaticMesh _staticmesh (Variables|Default|GetNewStaticMesh))
  (Components|Box|SetBoxExtent (Variables|Default|GetBox) (* (.BoxExtent (Collision|GetComponentBounds _staticmesh)) 1.25) true))