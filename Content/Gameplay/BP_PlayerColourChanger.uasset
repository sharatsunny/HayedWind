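; BP_PlayerColourChanger is a Blueprint that drives a colour-change parameter from the player pawn's distance to its Cone component.
; Every Tick it takes the squared distance, normalizes it to a range, divides it by a constant and clamps it to 0–1.
; The result is written to the ColourChanger scalar in the ColourChanger Material Parameter Collection, rising as the player moves away.
; The clamped value is also printed on screen each frame.
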(event EventTick
  (params (DeltaSeconds :type Float%20%28single-precision%29))
  (bind _returnvalue (Game|Player|GetPlayerPawn 0))
  (bind _cone (Variables|Default|GetCone))
  (bind _returnvalue_2 (Transformation|GetActorLocation _returnvalue))
  (bind _returnvalue_3 (Transformation|GetWorldLocation _cone))
  (bind _returnvalue_4 (- _returnvalue_2 _returnvalue_3))
  (bind (_x _y _z) (Math|Vector|BreakVector _returnvalue_4))
  (bind _returnvalue_5 (Math|Float|Square _x))
  (bind _returnvalue_6 (Math|Float|Square _y))
  (bind _returnvalue_7 (Math|Float|Square _z))
  (bind _returnvalue_8 (+ _returnvalue_5 _returnvalue_6 _returnvalue_7))
  (bind _returnvalue_9 (Math|Float|NormalizetoRange _returnvalue_8 2.5e+02 1.2e+03))
  (bind _returnvalue_10 (/ _returnvalue_9 1e+03))
  (bind _returnvalue_11 (Math|Float|Clamp(Float) _returnvalue_10))
  (Development|PrintString (Utilities|String|ToString(Float) _returnvalue_11))
  (Rendering|Material|SetScalarParameterValue "/Game/Mannequin/Character/Materials/ColourChanger.ColourChanger" "ColourChanger" (Math|Float|Lerp 0.0 1.0 _returnvalue_11) :!class /Script/Engine.KismetMaterialLibrary))

(fn ConstructionScript)