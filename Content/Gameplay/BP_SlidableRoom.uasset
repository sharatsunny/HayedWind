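; BP_SlidableRoom is a room actor built from nine static mesh components, with one mesh swappable per instance.
; Its construction script gathers the components into an array, picks the one at MeshIndex and assigns NewMesh to it.
; The event graph holds only disabled placeholder events, so the Blueprint itself contains no runtime or sliding logic.
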(event EventBeginPlay)

(event Collision|EventActorBeginOverlap
  (params (OtherActor :type Actor%20Object%20Reference)))

(event EventTick
  (params (DeltaSeconds :type Float%20%28single-precision%29)))

(fn ConstructionScript
  (Components|StaticMesh|SetStaticMesh (Utilities|Array|Get(acopy) (Utilities|Array|MakeArray (Variables|Default|GetStaticMesh) (Variables|Default|GetStaticMesh1) (Variables|Default|GetStaticMesh2) (Variables|Default|GetStaticMesh3) (Variables|Default|GetStaticMesh4) (Variables|Default|GetStaticMesh5) (Variables|Default|GetStaticMesh6) (Variables|Default|GetStaticMesh7) (Variables|Default|GetStaticMesh8)) (Variables|Default|GetMeshIndex)) (Variables|Default|GetNewMesh)))