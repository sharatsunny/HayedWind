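; Pressure-plate style actor in the intro level that changes fog density when the player stands on it.
; Overlap plays a timeline that lowers the block mesh, reversing if the overlap ends before the block is fully down.
; Once down, Tick calls FadeFog every frame while the player remains, restarting the fog density timeline.
; The same fog timeline also plays in reverse two seconds after BeginPlay.
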(event Custom|FadeFog
  (bind _fadefogalpha (Timeline|FogIntentsity PlayFromStart)
    (:Update
      (Class|ExponentialHeightFogComponent|SetFogDensity (Variables|/Script/Engine.ExponentialHeightFog|GetComponent (Variables|Default|GetFogComponent)) _fadefogalpha))))

(event Collision|EventActorBeginOverlap
  (params (OtherActor :type Actor%20Object%20Reference))
  (bind _staticmesh (Variables|Default|GetStaticMesh))
  (Variables|Default|SetIsCollided (== OtherActor (Game|GetPlayerCharacter 0)))
  (if (Variables|Default|GetIsBlockFinished)
    (Variables|Default|SetIsCollided false)
    (else
      (bind _movedowntrack (Timeline|MoveBlockDown PlayFromStart)
        (:Update
          (Transformation|SetRelativeLocation _staticmesh (Math|Vector|MakeVector 0.0 0.0 _movedowntrack) false false)
          (Variables|Default|SetIsBlockFinished (== (.z (Variables|/Script/Engine.SceneComponent|GetRelativeLocation _staticmesh)) -3e+01)))
        (:Finished
          (Development|PrintString "Hello"))))))

(event EventTick
  (params (DeltaSeconds :type Float%20%28single-precision%29))
  (if (Variables|Default|GetIsCollided)
    (if (Variables|Default|GetIsBlockFinished)
      (CallFunction|FadeFog))))

(event Collision|EventActorEndOverlap
  (params (OtherActor :type Actor%20Object%20Reference))
  (bind _staticmesh (Variables|Default|GetStaticMesh))
  (Variables|Default|SetIsCollided false)
  (if (not (Variables|Default|GetIsBlockFinished))
    (bind _movedowntrack (Timeline|MoveBlockDown Reverse)
      (:Update
        (Transformation|SetRelativeLocation _staticmesh (Math|Vector|MakeVector 0.0 0.0 _movedowntrack) false false)
        (Variables|Default|SetIsBlockFinished (== (.z (Variables|/Script/Engine.SceneComponent|GetRelativeLocation _staticmesh)) -3e+01)))
      (:Finished
        (Development|PrintString "Hello")))))

(event EventBeginPlay
  (Utilities|FlowControl|Delay 2.0)
  (bind _fadefogalpha (Timeline|FogIntentsity ReverseFromEnd)
    (:Update
      (Class|ExponentialHeightFogComponent|SetFogDensity (Variables|/Script/Engine.ExponentialHeightFog|GetComponent (Variables|Default|GetFogComponent)) _fadefogalpha))))

(fn ConstructionScript)