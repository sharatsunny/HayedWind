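; BP_RestartGame is a trigger that ends a level when the ThirdPersonCharacter overlaps its box, then opens NextLevel.
; It acts only if NextLevel differs from the current level, fading camera and audio out over FadeDuration.
; After the fade, it shows UI_DeathHud in Level_EndBad or UI_LoveHud in any other level.
; Each screen holds for its own fixed delay before all widgets are removed and the level loads.
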(event OnComponentBeginOverlap(Box)
  (params (OverlappedComponent :type Primitive%20Component%20Object%20Reference) (OtherActor :type Actor%20Object%20Reference) (OtherComp :type Primitive%20Component%20Object%20Reference) (OtherBodyIndex :type Integer) (bFromSweep :type Boolean) (SweepResult :type Hit%20Result%20Structure%20%28by%20ref%29))
  (bind _nextlevel (Variables|Default|GetNextLevel))
  (bind _fadeduration (Variables|Default|GetFadeDuration))
  (Utilities|Casting|CastToThirdPersonCharacter OtherActor)
  (bind _returnvalue (Game|GetCurrentLevelName true))
  (if (not (Utilities|Enum|Equal(Enum) _returnvalue (Utilities|String|ToString(Name) _nextlevel)))
    (CameraFades|StartCameraFade :self (Game|GetPlayerCameraManager 0) :ToAlpha 1.0 :Duration _fadeduration :bShouldFadeAudio true :bHoldWhenFinished true)
    (Utilities|FlowControl|Delay _fadeduration)
    (if (Utilities|Enum|Equal(Enum) _returnvalue "Level_EndBad")
      (bind _returnvalue_2 (UserInterface|CreateWidget "/Game/UMG/UI_DeathHud.UI_DeathHud_C"))
      (UserInterface|Viewport|AddtoViewport _returnvalue_2 0)
      (Utilities|FlowControl|Delay 4.0)
      (Viewport|RemoveAllWidgets)
      (Game|OpenLevel(byName) _nextlevel)
      (else
        (bind _returnvalue_3 (UserInterface|CreateWidget "/Game/UMG/UI_LoveHud.UI_LoveHud_C"))
        (UserInterface|Viewport|AddtoViewport _returnvalue_3 0)
        (Utilities|FlowControl|Delay 7.0)
        (Viewport|RemoveAllWidgets)
        (Game|OpenLevel(byName) _nextlevel)))))

(fn ConstructionScript)